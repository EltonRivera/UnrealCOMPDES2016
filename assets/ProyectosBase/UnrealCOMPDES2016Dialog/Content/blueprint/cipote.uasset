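; Cipote is a Paper2D flipbook character that talks as either a boy or a girl, depending on the game's gender setting.
; Its Habla function reads IsGirl from the gameData GameInstance and switches to that gender's talking or non-talking flipbook.
; It then plays the matching 2D sound and returns its duration plus a short padding.
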(fn `habla`
  (params (habla :type Boolean) (soundBoy :type "SoundBase Object Reference") (soundGirl :type "SoundBase Object Reference"))
  (returns (duration :type "Float (double-precision)"))
  (bind _rendercomponent (`self.RenderComponent`))
  ;[1 1 1] Cambio de animaciones
  (bind _asgame_data (cast `/Game/blueprint/gameData` (`GameplayStatics.GetGameInstance`)))
  (if (`/Game/blueprint/gameData.isGirl` _asgame_data)
    (`PaperFlipbookComponent.SetFlipbook` _rendercomponent (select `bool` habla :`false` "/Game/flipbooks/girlNoTalk.girlNoTalk" :`true` "/Game/flipbooks/girlTalk.girlTalk" :!type "PaperFlipbook Object Reference"))
    (`GameplayStatics.PlaySound2D` soundGirl)
    (return (+ (`SoundBase.Duration` soundGirl) 0.5))
    (else
      (`PaperFlipbookComponent.SetFlipbook` _rendercomponent (select `bool` habla :`false` "/Game/flipbooks/boyNoTalk.boyNoTalk" :`true` "/Game/flipbooks/boyTalk.boyTalk" :!type "PaperFlipbook Object Reference"))
      (`GameplayStatics.PlaySound2D` soundBoy)
      (return (+ (`SoundBase.Duration` soundBoy) 0.5)))))

(fn `UserConstructionScript`)