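; Selectable geometric-figure actor that awards score when the player clicks or touches it.
; A click on its sprite or a touch on the actor runs the same logic, guarded by EsActivo so it fires only once.
; It briefly enlarges the sprite as feedback, restores its scale after a short delay, then calls SumarPuntuacion on the Puntaje reference.
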(event `self.SpriteFGeometrica.OnClicked`
  (params (TouchedComponent :type "PrimitiveComponent Object Reference"))
  (if (not (`self.EsActivo`)) :!label _label
    (set `self.EsActivo` true)
    (`SceneComponent.SetRelativeScale3D` (`self.SpriteFGeometrica`) (1.5 1.0 1.5))
    (`KismetSystemLibrary.Delay` 0.5)
    (`SceneComponent.SetRelativeScale3D` (`self.SpriteFGeometrica`) (1.0 1.0 1.0))
    (`/Game/blueprint/Puntuacion.SumarPuntuacion` (`self.Puntaje`))))

(event `self.ReceiveActorOnInputTouchBegin`
  (params (FingerIndex :type "ETouchIndex Enum" :default "Touch1"))
  (goto _label))

(fn `UserConstructionScript`)